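; Performance benchmark actor that measures average frame rate as waves of actors are spawned, then quits the game after a set number of steps.
; A DoN loop with delays asks ActorSpawner for another wave each step interval.
; Tick counts frames against a countdown timer, writes each step's average FPS to a JSON object and saves it to FPSData.json in the game source directory.
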(event `self.ReceiveBeginPlay`
  (`|ExecutionSequence`
    (:`then_0`
      ;[1 0.2837 0.7306] Set Save File path
      (set `self.filePath` (make `FilePath` (`KismetStringLibrary.Concat_StrStr` (`BlueprintPathsLibrary.GameSourceDir`) "FPSData.json")))
      ;[0.1824 0.305 1] Clear File
      (bind _outjsonobject (`JsonBlueprintFunctionLibrary.FromString` ""))
      (set `self.jsonObject` _outjsonobject))
    (:`then_1`
      (`self.ResetTimer`)
      (`KismetSystemLibrary.Delay` 0.01)
      ;[0.3807 0.5609 1] Spawn Actors
      (`/Game/Blueprints/BP_ActorSpawner.SpawnActorWave` (`self.actorSpawner`))
      (bind _counter (`/Engine/EditorBlueprintResources/StandardMacros.Do N` (`self.totalSteps`) :!label _label)
        (:`Exit`
          (set `self.currentTestStep` _counter)
          (`KismetSystemLibrary.Delay` (`self.stepLength`))
          (`/Game/Blueprints/BP_ActorSpawner.SpawnActorWave` (`self.actorSpawner`))
          (goto _label))))))

(event `self.ReceiveTick`
  (params (DeltaSeconds :type "Float (single-precision)"))
  (`|ExecutionSequence`
    (:`then_0`
      ;[0.2872 1 0.6889] Count Frame
      (bind _result (`/Engine/EditorBlueprintResources/StandardMacros.IncrementInt` (`self.countedFrames`))
        (:`  `
          (set `self.countedFrames` _result))))
    (:`then_1`
      ;[0.3687 0.8427 0.3687] Update Timer
      (set `self.stepTimer` (- (`self.stepTimer`) DeltaSeconds)))
    (:`then_2`
      ;[1 0.2031 0.2031] Timer done check
      (if (< (`self.stepTimer`) 0.0)
        (`self.ResetTimer`)
        ;[0.9366 1 0.5925] ReportFrameRate
        (`|ExecutionSequence`
          (:`then_0`
            (`|SetJsonField` (`self.jsonObject`) (`KismetStringLibrary.Concat_StrStr` (`KismetStringLibrary.Conv_IntToString` (`self.currentTestStep`)) " Average FPS: ") (/ (`self.countedFrames`) (`self.stepLength`)))
            ;;[1 0.5752 0.4159] Save To JSON
            (`JsonBlueprintFunctionLibrary.ToFile` (`self.jsonObject`) (`self.filePath`))
            ;[1 0.2554 0.2892] Quit Game Condition
            (if (>= (`self.currentTestStep`) (`self.totalSteps`))
              (`KismetSystemLibrary.QuitGame` null "Quit")))
          (:`then_1`
            ;;[0.5251 0.9582 1] Reset Counted Frames
            (set `self.countedFrames` 0)))))))

(fn `ResetTimer`
  (set `self.stepTimer` (`self.stepLength`))
  (return))

(fn `UserConstructionScript`)