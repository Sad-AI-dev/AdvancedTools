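; BP_SimpleMoverCube is a cube actor that each tick moves toward another cube of its class, then jitters randomly.
; It gathers all mover cubes over one unit away and steps at MoveSpeed toward the selected target.
; FindNearestActor's inverted comparison actually selects the farthest cube, and the snap-to-target check measures Others[0] instead of the target.
; MoveRandomOffset then adds a random offset within ±MaxOffset per axis.
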(event `self.ReceiveTick`
  (params (DeltaSeconds :type "Float (single-precision)"))
  (`self.MoveTowardsNearestNeighbour`)
  (`self.MoveRandomOffset`))

(fn `FindNearestActor`
  (params (Others :type "Array of Actor Object Reference"))
  (returns (Closest :type "Actor Object Reference"))
  (locals (ClosestIndex :type Integer) (ClosestDistance :type "Float (double-precision)"))
  (`|ExecutionSequence`
    (:`then_0`
      ;[0.3206 1 0.7143] Initialize Vars
      (`|ExecutionSequence`
        (:`then_0`
          (set `local.ClosestIndex` 0))
        (:`then_1`
          (set `local.ClosestDistance` (`KismetMathLibrary.Vector_Distance` (`self.K2_GetActorLocation`) (`self.K2_GetActorLocation` (`|GetArrayItem` (`local.Others`))))))))
    (:`then_1`
      ;[1 0.3577 0.4475] Find Closest
      (for (_array_element _array_index) (`local.Others`)
        (bind _returnvalue (`KismetMathLibrary.Vector_Distance` (`self.K2_GetActorLocation` _array_element) (`self.K2_GetActorLocation`)))
        ;;[0.4026 1 0.3427] Distance Check
        (if (< (`local.ClosestDistance`) _returnvalue)
          (set `local.ClosestDistance` _returnvalue)
          (set `local.ClosestIndex` _array_index))))
    (:`then_2`
      ;[0.9979 0.3253 1] Report Result
      (return (`|GetArrayItem` (`local.Others`) (`local.ClosestIndex`))))))

(fn `MoveRandomOffset`
  (bind (_x _y _z) (`KismetMathLibrary.BreakVector3f` (`self.maxOffset`)))
  (`self.K2_SetActorLocation` (+ (`self.K2_GetActorLocation`) (- (* (`KismetMathLibrary.MakeVector` (* _x (`KismetMathLibrary.RandomFloat`)) (* _y (`KismetMathLibrary.RandomFloat`)) (* _z (`KismetMathLibrary.RandomFloat`))) 2.0) (`self.maxOffset`)))))

(fn `MoveTowardsNearestNeighbour`
  (locals (others :type "Array of Actor Object Reference") (targetActor :type "Actor Object Reference"))
  (`|ExecutionSequence`
    (:`then_0`
      ;[0.6452 0.8759 1] Get and Sort List of other mover cubes based on distance to self
      (bind _outactors (`GameplayStatics.GetAllActorsOfClass` "BP_SimpleMoverCube_C"))
      (for _array_element _outactors
        ;;[0.1085 0.2779 1] Add others to list
        (if (> (`self.GetDistanceTo` _array_element) 1.0)
          (`KismetArrayLibrary.Array_Add` (`local.others`) _array_element)))
      (if (> (`KismetArrayLibrary.Array_Length` (`local.others`)) 0)
        ;;[0.2269 0.8457 1] Set Closest
        (bind _closest (`self.FindNearestActor` (`local.others`)))
        (set `local.targetActor` _closest)))
    (:`then_1`
      (if (> (`KismetArrayLibrary.Array_Length` (`local.others`)) 0)
        ;[0.9749 0.7324 1] Move towards closest
        (if (<= (`self.GetDistanceTo` (`|GetArrayItem` (`local.others`))) (* (`self.moveSpeed`) (`GameplayStatics.GetWorldDeltaSeconds`)))
          ;;[0.6417 1 0.5546] Set to target position
          (`self.K2_SetActorLocation` (`self.K2_GetActorLocation` (`local.targetActor`)))
          (else
            ;;[0.5995 1 0.5742] Move towards target position
            (`self.K2_SetActorLocation` (+ (`self.K2_GetActorLocation`) (* (`KismetMathLibrary.Normal` (- (`self.K2_GetActorLocation` (`local.targetActor`)) (`self.K2_GetActorLocation`))) (* (`self.moveSpeed`) (`GameplayStatics.GetWorldDeltaSeconds`)))))))))))

(fn `UserConstructionScript`)