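; BP_MoverCube is an actor that each tick moves toward another mover cube while jittering randomly.
; MoveTowardsNearestNeighbour collects cubes farther than 100 units away, orders them by distance through an insertion sort in SortListBasedOnDistance, and targets the first.
; It steps toward that target at MoveSpeed scaled by delta time, snapping onto it when within one step.
; MoveRandomOffset then adds a centred random displacement sized by MaxOffset, independent of frame time.
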(event `self.ReceiveTick`
  (params (DeltaSeconds :type "Float (single-precision)"))
  (`self.MoveTowardsNearestNeighbour`)
  (`self.MoveRandomOffset`))

(fn `MoveRandomOffset`
  (bind _returnvalue (`KismetMathLibrary.RandomFloat`))
  (bind (_maxoffset_x _maxoffset_y _maxoffset_z) (break `Vector3f` (`self.maxOffset`)))
  (`self.K2_SetActorLocation` (+ (`self.K2_GetActorLocation`) (`KismetMathLibrary.MakeVector` (- (* _returnvalue _maxoffset_x) (/ _maxoffset_x 2.0)) (- (* _returnvalue _maxoffset_y) (/ _maxoffset_y 2.0)) (- (* _returnvalue _maxoffset_z) (/ _maxoffset_z 2.0))))))

(fn `MoveTowardsNearestNeighbour`
  (locals (others :type "Array of Actor Object Reference") (targetActor :type "Actor Object Reference"))
  (`|ExecutionSequence`
    (:`then_0`
      ;[0.6452 0.8759 1] Get and Sort List of other mover cubes based on distance to self
      (bind _outactors (`GameplayStatics.GetAllActorsOfClass` "BP_MoverCube_C"))
      (for _array_element _outactors
        ;;[0.1085 0.2779 1] Add others to list
        (if (> (`self.GetDistanceTo` _array_element) 100.0)
          (`KismetArrayLibrary.Array_Add` (`local.others`) _array_element)))
      (if (> (`KismetArrayLibrary.Array_Length` (`local.others`)) 0)
        ;;[0.2269 0.8457 1] Sort List
        (bind _sortedlist (`self.SortListBasedOnDistance` (`local.others`)))
        (bind _output_get (set `local.others` _sortedlist))
        (set `local.targetActor` (`|GetArrayItem` _output_get))))
    (:`then_1`
      (if (> (`KismetArrayLibrary.Array_Length` (`local.others`)) 0)
        ;[0.9749 0.7324 1] Move towards closest
        (if (<= (`self.GetDistanceTo` (`|GetArrayItem` (`local.others`))) (* (`self.moveSpeed`) (`GameplayStatics.GetWorldDeltaSeconds`)))
          ;;[0.6417 1 0.5546] Set to target position
          (`self.K2_SetActorLocation` (`self.K2_GetActorLocation` (`local.targetActor`)))
          (else
            ;;[0.5995 1 0.5742] Move towards target position
            (`self.K2_SetActorLocation` (+ (`self.K2_GetActorLocation`) (* (`KismetMathLibrary.Normal` (- (`self.K2_GetActorLocation` (`local.targetActor`)) (`self.K2_GetActorLocation`))) (* (`self.moveSpeed`) (`GameplayStatics.GetWorldDeltaSeconds`)))))))))))

(fn `SortListBasedOnDistance`
  (params (targetList :type "Array of Actor Object Reference"))
  (returns (SortedList :type "Array of Actor Object Reference"))
  (locals (currentTarget :type "Actor Object Reference") (currentIndex :type Integer) (targetDistance :type "Float (double-precision)") (SortingList :type "Array of Actor Object Reference"))
  (bind _currentindex (`local.currentIndex`))
  (for (_array_element _array_index) targetList
    (set `local.currentTarget` _array_element)
    (set `local.currentIndex` _array_index)
    ;[0.5597 1 0.4905] Get Distance
    (set `local.targetDistance` (`self.GetDistanceTo` (`local.currentTarget`)))
    (while (and (> (`self.GetDistanceTo` (`|GetArrayItem` (`local.SortingList`) (- _currentindex 1))) (`local.targetDistance`)) (> _currentindex 0))
      ;[1 1 1] Lower Index
      (set `local.currentIndex` (- (`local.currentIndex`) 1)))
    ;[1 1 1] Insert target at index
    (`KismetArrayLibrary.Array_Insert` (`local.SortingList`) (`local.currentTarget`) (`local.currentIndex`)))
  (return (`local.SortingList`)))

(fn `UserConstructionScript`)