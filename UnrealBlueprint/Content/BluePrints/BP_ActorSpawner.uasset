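; Spawner actor that creates waves of a configurable actor class, laid out on a stepped lattice.
; SpawnActorWave calls CreateNextActor over the AmountToSpawn range, advancing a running TotalSpawned index across waves.
; Each index maps to Y modulo ten, Z per ten and X per hundred (Z never wraps), scaled by SpawnOffset from SpawnPos.
; BeginPlay only decrements AmountToSpawn; nothing here triggers a wave.
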(event `self.ReceiveBeginPlay`
  (`/Engine/EditorBlueprintResources/StandardMacros.DecrementInt` (`self.amountToSpawn`)))

(fn `CreateNextActor`
  (params (num :type Integer))
  (returns (`created Actor` :type "Actor Object Reference"))
  (locals (finalSpawnPos :type "Vector Structure"))
  ;[0.4737 0.563 1] Spawn Actor
  (bind _returnvalue (`|SpawnActorFromClass` (`self.actorToSpawn`) (`self.GetTransform`) "Undefined" "OverrideRootScale" null null))
  (`self.K2_SetActorLocation` _returnvalue (+ (* (`KismetMathLibrary.MakeVector` (`KismetMathLibrary.Conv_IntToDouble` (`KismetMathLibrary.FFloor` (/ (`KismetMathLibrary.Conv_IntToDouble` num) 100.0))) (`KismetMathLibrary.Conv_IntToDouble` (mod num 10)) (`KismetMathLibrary.Conv_IntToDouble` (`KismetMathLibrary.FFloor` (/ (`KismetMathLibrary.Conv_IntToDouble` num) 10.0)))) (`self.spawnOffset`)) (`self.spawnPos`)) false false)
  (return _returnvalue))

(fn `SpawnActorWave`
  (for _ (range (+ (`self.amountToSpawn`) 1))
    (`self.CreateNextActor` (`self.totalSpawned`))
    (bind _result (`/Engine/EditorBlueprintResources/StandardMacros.IncrementInt` (`self.totalSpawned`))
      (:`  `
        (set `self.totalSpawned` _result)))))

(fn `UserConstructionScript`)